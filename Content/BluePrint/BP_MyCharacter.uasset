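; Character Blueprint that adds crouch and roll actions through Enhanced Input and shows a stamina widget.
; BeginPlay creates WBP_Stamina and adds it to the viewport, with no stamina logic in this graph.
; Crouch input toggles Crouch and UnCrouch through a FlipFlop.
; Roll input plays a one-shot mesh animation while the Movement timeline sets velocity along actor forward, scaled by the anim instance's MoveLength.
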(event `EnhancedInput|/Game/Input/IA_Crouch`
  (params (ActionValue :type Boolean) (ElapsedSeconds :type "Float (double-precision)") (TriggeredSeconds :type "Float (double-precision)") (InputAction :type "InputAction Object Reference" :default "/Game/Input/IA_Crouch.IA_Crouch"))
  (:`Started`
    (`/Engine/EditorBlueprintResources/StandardMacros.FlipFlop`
      (:`A`
        (`self.Crouch`))
      (:`B`
        (`self.UnCrouch`)))))

(event `self.ReceiveBeginPlay`
  (bind _returnvalue (`|CreateWidget` "/Game/BluePrint/WBP_Stamina.WBP_Stamina_C"))
  (`UserWidget.AddToViewport` _returnvalue 0))

(event `EnhancedInput|/Game/Input/IA_Roll`
  (params (ActionValue :type Boolean) (ElapsedSeconds :type "Float (double-precision)") (TriggeredSeconds :type "Float (double-precision)") (InputAction :type "InputAction Object Reference" :default "/Game/Input/IA_Roll.IA_Roll"))
  (:`Triggered`
    (`SkeletalMeshComponent.PlayAnimation` (`self.Mesh`) null false)
    (`Timeline|Movement` :!via `PlayFromStart`
      (:`Update`
        (set `MovementComponent.Velocity` (* (`self.GetActorForwardVector`) (`MyAnimInstance.MoveLength` (`self.MyAnimInstance`))) (`self.CharacterMovement`))))))

(fn `UserConstructionScript`)